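; Chest actor that highlights itself through custom depth stencil values on its body and cover meshes.
; Cursor hover on either mesh, or holding the Highlight input, sets selection flags and calls UpdateChestState.
; That function writes the configurable stencil value to both meshes while either flag is set, and zero otherwise.
; SetCustomStencilValue changes the stored stencil ID without refreshing the meshes.
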(event `self.ReceiveBeginPlay`
  (`self.UpdateChestState`))

(event `self.Chest_Chest.OnBeginCursorOver`
  (params (TouchedComponent :type "PrimitiveComponent Object Reference"))
  (set `self.SelectedChest` true)
  (`self.UpdateChestState` :!label _label))

(event `self.Chest_Chest_cover.OnBeginCursorOver`
  (params (TouchedComponent :type "PrimitiveComponent Object Reference"))
  (set `self.SelectedChestCover` true)
  (goto _label))

(event `self.Chest_Chest.OnEndCursorOver`
  (params (TouchedComponent :type "PrimitiveComponent Object Reference"))
  (set `self.SelectedChest` false)
  (goto _label))

(event `self.Chest_Chest_cover.OnEndCursorOver`
  (params (TouchedComponent :type "PrimitiveComponent Object Reference"))
  (set `self.SelectedChestCover` false)
  (goto _label))

(event `InputAction|Highlight` :consume false
  (params (Key :type "Key Structure"))
  (:`Pressed`
    (set `self.SelectedChest` true)
    (set `self.SelectedChestCover` true)
    (`self.UpdateChestState` :!label _label_2))
  (:`Released`
    (set `self.SelectedChest` false)
    (set `self.SelectedChestCover` false)
    (goto _label_2)))

(fn `SetCustomStencilValue`
  (params (StencilID :type Integer))
  (set `self.CustomStencilValue` StencilID))

(fn `UpdateChestState`
  (if (or (`self.SelectedChestCover`) (`self.SelectedChest`))
    (`PrimitiveComponent.SetCustomDepthStencilValue` (`self.Chest_Chest_cover`) (`self.CustomStencilValue`))
    (`PrimitiveComponent.SetCustomDepthStencilValue` (`self.Chest_Chest`) (`self.CustomStencilValue`))
    (else
      (`PrimitiveComponent.SetCustomDepthStencilValue` (`self.Chest_Chest`) 0)
      (`PrimitiveComponent.SetCustomDepthStencilValue` (`self.Chest_Chest_cover`) 0))))

(fn `UserConstructionScript`)